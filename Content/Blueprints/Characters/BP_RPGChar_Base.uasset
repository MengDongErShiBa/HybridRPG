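; BP_RPGChar_Base is a base RPG character Blueprint that supports interaction and data-table-driven dialogue.
; Interaction runs StartInteraction on the instigator and itself, locking interaction and halting its movement, then sends the current DT_Dialogue row to the GM_RPG HUD widget.
; ShowNextLine follows each row's NextRow link, resetting to the starting row and returning false when the chain ends.
; FinishInteraction releases the character's lock.
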(event EventBeginPlay
  (Rendering|SetCastShadow (Variables|Default|Get%20DialogueIndicator) false)
  (Variables|Default|SetResetRowName (Variables|Default|GetCurrentRowName))
  (bind _asgm_rpg (Utilities|Casting|CastToGM_RPG (Game|GetGameMode)))
  (Variables|Default|SetGameMode _asgm_rpg))

(event Collision|EventActorBeginOverlap
  (params (OtherActor :type Actor%20Object%20Reference)))

(event EventTick
  (params (DeltaSeconds :type Float%20%28single-precision%29)))

(event EventFinishInteraction
  (CallFunction|EndInteraction))

(event EventInteraction
  (params (Instigator :type BP%20RPG%20Char%20Base%20Object%20Reference))
  (if (not (== (Variables|Default|GetCurrentRowName) "None"))
    (CallFunction|StartInteraction Instigator Instigator)
    (CallFunction|StartInteraction Instigator)
    (CallFunction|ShowDialogueLine)))

(fn ConstructionScript)

(fn ShowDialogueLine
  (bind _returnvalue (Utilities|GetDataTableRow "/Game/DataTables/DT_Dialogue.DT_Dialogue" (Variables|Default|GetCurrentRowName))
    (:then
      (Default|ShowDialogue (Variables|/Game/Blueprints/GM_RPG.GM_RPG_C|GetHUDWidget (Variables|Default|GetGameMode)) self (Variables|Default|GetSpeaker%20Name) (.DialogueText (Utilities|Struct|BreakS_DialogueData _returnvalue)))
      (Variables|Default|SetNext%20Row (.NextRow (Utilities|Struct|BreakS_DialogueData _returnvalue)))
      (return))))

(fn StartInteraction
  (params (Interactinstigator :type Actor%20Object%20Reference))
  (Variables|Default|SetIsInteractionLocked true)
  (Components|Movement|StopMovementImmediately (Variables|Character|GetCharacterMovement)))

(fn EndInteraction
  (Variables|Default|SetIsInteractionLocked false))

(fn ShowNextLine
  (if (Utilities|Array|IsEmpty (Variables|Default|GetNext%20Row))
    (Variables|Default|SetCurrentRowName (Variables|Default|GetResetRowName))
    (return false)
    (else
      (Variables|Default|SetCurrentRowName (Utilities|String|StringToName (Variables|Default|GetNext%20Row)))
      (CallFunction|ShowDialogueLine)
      (return true))))